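; AI opponent character for a fighting game, picking its mesh setup, animation Blueprint and montage set from the current level.
; A looping timer randomly chooses moves, jumps, blocks, combo punches or charged attacks based on player proximity, while Tick applies side movement and hurt reactions.
; Montage-driven attacks set the damage, including a one-time boosted super.
; HitCheck damages overlapping players and updates health UI; blocking negates incoming damage.
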(event OnComponentBeginOverlap(PlayerClose)
  (params (OverlappedComponent :type Primitive%20Component%20Object%20Reference) (OtherActor :type Actor%20Object%20Reference) (OtherComp :type Primitive%20Component%20Object%20Reference) (OtherBodyIndex :type Integer) (bFromSweep :type Boolean) (SweepResult :type Hit%20Result%20Structure%20%28by%20ref%29))
  ;[1 1 1] Is Player Close?
  (if (!= OtherActor self)
    (Variables|AIDetections|SetbIsPlayerClose true)))

(event OnComponentEndOverlap(PlayerClose)
  (params (OverlappedComponent :type Primitive%20Component%20Object%20Reference) (OtherActor :type Actor%20Object%20Reference) (OtherComp :type Primitive%20Component%20Object%20Reference) (OtherBodyIndex :type Integer))
  ;[1 1 1] Is Player Close?
  (if (!= OtherActor self)
    (Variables|AIDetections|SetbIsPlayerClose false)))

(event Custom|GameManager
  (bind _returnvalue (Math|Random|RandomIntegerinRange 0 100))
  ;[1 1 1] AI Logic
  (if (Variables|Default|GetStart)
    (if (not (CallFunction|Parameters))
      (if (Variables|AIDetections|GetbIsPlayerClose)
        (switch int (Math|Random|RandomIntegerinRange 0 4)
          (:0
            (CallFunction|ChargeAttack)
            (Variables|Default|SetbNeedsToMove false :!label _label))
          (:1
            (CallFunction|Attack1P)
            (goto _label))
          (:2
            (CallFunction|Block)
            (goto _label))
          (:3
            (Variables|Default|SetbNeedsToMove true)
            (Variables|Default|SetMoveDirection 1.0))
          (:4
            (Character|Jump :!label _label_2)
            (Variables|Default|SetbNeedsToMove true :!label _label_3)
            (Variables|Default|SetMoveDirection -1.0)
            (CallFunction|Attack1P)))
        (elif (<= _returnvalue 40)
          (goto _label_3)
          (elif (and (> _returnvalue 40) (<= _returnvalue 70))
            (goto _label_2)
            (else
              (Variables|Default|SetbNeedsToMove false))))))))

(event Custom|Attack1P
  ;[1 1 1] Attack1P
  (if (not (CallFunction|Parameters))
    (Variables|Default|SetAttacking true)
    (Animation|Montage|PlayMontage (Variables|Character|GetMesh) (Utilities|Select :Index (+ (Variables|Default|GetAttackCount) (* (Variables|Default|GetPlayerNumber) 3)) :Option%200 "/Game/Paul/Character1/Model/Animations/Montage/Punching_Montage.Punching_Montage" :Option%201 "/Game/Paul/Character1/Model/Animations/Montage/Punching2_Montage.Punching2_Montage" :Option%202 "/Game/Paul/Character1/Model/Animations/Montage/Hook_Montage.Hook_Montage" :Option%203 "/Game/Paul/Character1/Model2/Animations/Montage/Punch1_Montage.Punch1_Montage" :Option%204 "/Game/Paul/Character1/Model2/Animations/Montage/Punch2_Montage.Punch2_Montage" :Option%205 "/Game/Paul/Character1/Model2/Animations/Montage/Punch3_Montage.Punch3_Montage")
      (:then
        (Variables|Default|SetAttackCount (Math|Integer|Clamp(Integer) (+ (Variables|Default|GetAttackCount) 1) 0 2))
        (Variables|Damage|SetDamageToDeal (* (Variables|Damage|GetAttack1PDamage) (Utilities|Select :Index (Variables|Default|GetAttackCount) :Option%200 1.0 :Option%201 2.0 :Option%202 3.0)))
        (if (<= (Variables|Default|GetAttackCount) 2)
          (if (Math|Random|RandomBool)
            (Utilities|FlowControl|Delay 0.7)
            (CallFunction|Combo))))
      (:OnCompleted
        (Variables|Default|SetAttackCount 0 :!label _label)
        (Development|SetHiddeninGame (Variables|Default|GetKickHitbox) true false))
      (:OnInterrupted
        (Utilities|FlowControl|RetriggerableDelay 2.2)
        (Variables|Default|SetAttacking false)
        (goto _label)))))

(event Custom|ChargeAttack
  ;[1 1 1] ChargeAttack
  (Utilities|FlowControl|Sequence
    (:then_0
      (if (not (CallFunction|Parameters))
        (Variables|Default|SetAttacking true)
        (Animation|Montage|PlayMontage (Variables|Character|GetMesh) (Utilities|Select :Index (Variables|Default|GetPlayerNumber) :Option%200 "/Game/Paul/Character1/Model/Animations/Montage/charging_Montage.charging_Montage" :Option%201 "/Game/Paul/Character1/Model2/Animations/Montage/StartCharged_Montage.StartCharged_Montage" :Option%202 0)
          (:then
            (Variables|Default|Setcharging true)))))
    (:then_1
      (if (Variables|Default|GetbSuperPowerUsed)
        (Rendering|SetVisibility (Variables|Default|GetPointLight) false false :!label _label)
        (Variables|Damage|SetAttack2PDamage 2e+01)
        (Utilities|FlowControl|Delay (Math|Random|RandomFloatinRange 0.0 0.5))
        (CallFunction|Attack2P)
        (elif (Math|Random|RandomBool)
          (Utilities|FlowControl|Delay 0.99)
          (Rendering|SetVisibility (Variables|Default|GetPointLight) true false)
          (Variables|Damage|SetAttack2PDamage (* (Variables|Damage|GetAttack2PDamage) 3.0))
          (bind _output_get (Variables|Default|SetbSuperPowerUsed true))
          (Default|UseSuper (Variables|/Game/Paul/PC_PlayerController.PC_PlayerController_C|GetWB_Main (Variables|/Game/Paul/Character1/BP_FightingPlayer.BP_FightingPlayer_C|GetAs%20PC%20Player%20Controller (Variables|/Game/Paul/GM_FightingPlayer.GM_FightingPlayer_C|GetPlayer (Variables|References|GetGM)))) _output_get)
          (CallFunction|Attack2P)
          (else
            (goto _label)))))))

(event Custom|Combo
  ;[1 1 1] Attack1P
  (Variables|Default|SetAttacking true)
  (Animation|Montage|PlayMontage (Variables|Character|GetMesh) (Utilities|Select :Index (+ (Variables|Default|GetAttackCount) (* (Variables|Default|GetPlayerNumber) 3)) :Option%200 "/Game/Paul/Character1/Model/Animations/Montage/Punching_Montage.Punching_Montage" :Option%201 "/Game/Paul/Character1/Model/Animations/Montage/Punching2_Montage.Punching2_Montage" :Option%202 "/Game/Paul/Character1/Model/Animations/Montage/Hook_Montage.Hook_Montage" :Option%203 "/Game/Paul/Character1/Model2/Animations/Montage/Punch1_Montage.Punch1_Montage" :Option%204 "/Game/Paul/Character1/Model2/Animations/Montage/Punch2_Montage.Punch2_Montage" :Option%205 "/Game/Paul/Character1/Model2/Animations/Montage/Punch3_Montage.Punch3_Montage")
    (:then
      (Variables|Default|SetAttackCount (Math|Integer|Clamp(Integer) (+ (Variables|Default|GetAttackCount) 1) 0 2))
      (Variables|Damage|SetDamageToDeal (* (Variables|Damage|GetAttack1PDamage) (Utilities|Select :Index (Variables|Default|GetAttackCount) :Option%200 1.0 :Option%201 2.0 :Option%202 3.0)))
      (if (<= (Variables|Default|GetAttackCount) 2)
        (if (Math|Random|RandomBool)
          (Utilities|FlowControl|Delay 0.7)
          (CallFunction|Combo))))
    (:OnCompleted
      (Variables|Default|SetAttackCount 0 :!label _label)
      (Development|SetHiddeninGame (Variables|Default|GetKickHitbox) true false))
    (:OnInterrupted
      (Utilities|FlowControl|RetriggerableDelay 2.2)
      (Variables|Default|SetAttacking false)
      (goto _label))))

(event Custom|Attack2P
  ;[1 1 1] Attack2P
  (if (Variables|Default|GetAttacking)
    (if (Variables|Default|Getcharging)
      (Animation|Montage|PlayMontage (Variables|Character|GetMesh) (Utilities|Select :Index (Variables|Default|GetPlayerNumber) :Option%200 "/Game/Paul/Character1/Model/Animations/Montage/chargedattack_Montage.chargedattack_Montage" :Option%201 "/Game/Paul/Character1/Model2/Animations/Montage/EndCharged_Montage.EndCharged_Montage")
        (:then
          (Variables|Damage|SetDamageToDeal (Variables|Damage|GetAttack2PDamage))
          (Development|SetHiddeninGame (Variables|Default|GetKickHitbox) true false)
          (Utilities|FlowControl|Delay 0.2)
          (Rendering|SetVisibility (Variables|Default|GetPointLight) false false))
        (:OnCompleted
          (Variables|Default|SetAttacking false)
          (Variables|Default|Setcharging false))))))

(event Custom|Block
  ;[1 1 1] Block
  (if (not (CallFunction|Parameters))
    (Variables|Default|SetBlocking true)
    (Animation|Montage|PlayMontage (Variables|Character|GetMesh) (Utilities|Select :Index (Variables|Default|GetPlayerNumber) :Option%200 "/Game/Paul/Character1/Model/Animations/Montage/Blocking_Montage.Blocking_Montage" :Option%201 "/Game/Paul/Character1/Model2/Animations/Montage/StartBlock_Montage.StartBlock_Montage") 2.0
      (:then
        (Utilities|FlowControl|Delay (Math|Random|RandomFloatinRange 1.0 2.0))
        (CallFunction|ReleaseBlock)))))

(event Custom|ReleaseBlock
  ;[1 1 1] Block
  (Animation|Montage|PlayMontage (Variables|Character|GetMesh) (Utilities|Select :Index (Variables|Default|GetPlayerNumber) :Option%200 "/Game/Paul/Character1/Model/Animations/Montage/StopBlocking_Montage.StopBlocking_Montage" :Option%201 "/Game/Paul/Character1/Model2/Animations/Montage/EndBlock_Montage.EndBlock_Montage") 2.0
    (:OnCompleted
      (Variables|Default|SetBlocking false))))

(event EventBeginPlay
  ;[1 1 1] AI Logic
  (CallFunction|SetPlayer)
  (Variables|Default|SetCurrentHealth (Variables|Default|GetMaxHealth))
  (bind _asgm_fighting_player (Utilities|Casting|CastToGM_FightingPlayer (Game|GetGameMode)))
  (Variables|References|SetGM _asgm_fighting_player)
  (Variables|/Game/Paul/GM_FightingPlayer.GM_FightingPlayer_C|SetAI _asgm_fighting_player self)
  (bind _returnvalue (Utilities|Time|SetTimerbyEvent (delegate Custom|GameManager) 1.0 true 0.0 0.2))
  (Variables|Default|SetTimerHandleGameManger _returnvalue))

(event EventTick
  (params (DeltaSeconds :type Float%20%28single-precision%29))
  ;[1 1 1] Tick
  (CallFunction|FMove (Variables|Default|GetbNeedsToMove) (Variables|Default|GetMoveDirection))
  (if (Variables|Default|GetisHurt) ; Hurt Event
    (Utilities|FlowControl|DoOnce false :!label _label
      (:Completed
        (Animation|Montage|PlayMontage (Variables|Character|GetMesh) (Utilities|Select :Index (Variables|Default|GetPlayerNumber) :Option%200 "/Game/Paul/Character1/Model/Animations/Montage/TakingPunch_Montage.TakingPunch_Montage" :Option%201 "/Game/Paul/Character1/Model2/Animations/Montage/Hurt_Montage.Hurt_Montage")
          (:OnCompleted
            (Variables|Default|SetisHurt false)
            (goto _label Reset)))))))

(event Game|Damage|EventAnyDamage
  (params (Damage :type Float%20%28single-precision%29) (DamageType :type Damage%20Type%20Object%20Reference) (InstigatedBy :type Controller%20Object%20Reference) (DamageCauser :type Actor%20Object%20Reference))
  ;[1 1 1] Receive Damage
  (if (not (Variables|Default|GetBlocking))
    (Variables|Default|SetCurrentHealth (Math|Float|Clamp(Float) (- (Variables|Default|GetCurrentHealth) Damage) 0.0 1e+02))
    (Variables|Default|SetisHurt true)))

(fn ConstructionScript)

(fn HitCheck
  (params (Damage :type Float%20%28single-precision%29) (HitBox :type Primitive%20Component%20Object%20Reference))
  (for _array_element (Collision|GetOverlappingActors HitBox "/Game/Paul/Character1/BP_FightingPlayer.BP_FightingPlayer_C" :!class /Script/Engine.PrimitiveComponent)
    (if (!= _array_element self)
      (Game|Damage|ApplyDamage _array_element Damage 0 0)
      (bind _asbp_fighting_player (Utilities|Casting|CastToBP_FightingPlayer _array_element))
      (Default|UpdateHealthUI (Variables|/Game/Paul/PC_PlayerController.PC_PlayerController_C|GetWB_Main (Variables|/Game/Paul/Character1/BP_FightingPlayer.BP_FightingPlayer_C|GetAs%20PC%20Player%20Controller _asbp_fighting_player)) true (Variables|/Game/Paul/Character1/BP_FightingPlayer.BP_FightingPlayer_C|GetCurrentHealth _asbp_fighting_player)))))

(fn CheckLevel
  (bind _returnvalue (Game|GetCurrentLevelName true))
  (return (Utilities|Enum|Equal(Enum) _returnvalue "BunnyMap")))

(fn SetPlayer
  (bind _mesh (Variables|Character|GetMesh))
  (bind _mesh_2 (Variables|Character|GetMesh))
  (if (CallFunction|CheckLevel)
    ;[1 1 1] BOMB
    (Variables|/Script/Engine.SkeletalMeshComponent|SetSkeletalMeshAsset _mesh "/Game/Paul/Character1/Model2/T-Pose.T-Pose")
    (Class|SkeletalMeshComponent|SetAnimClass _mesh "/Game/Paul/Character1/ABP_FightingAI2.ABP_FightingAI2_C")
    (Variables|Default|SetPlayerNumber 1)
    (Transformation|SetRelativeTransform _mesh_2 (Math|Transform|MakeTransform "0.000000,0.000000,-66.447029" "0.000000,-89.999999,0.000000" "0.500000,0.500000,0.500000") false false)
    (return)
    (else
      ;[1 1 1] BUNNY
      (Variables|/Script/Engine.SkeletalMeshComponent|SetSkeletalMeshAsset _mesh "/Game/Paul/Character1/Model/T-Pose.T-Pose")
      (Class|SkeletalMeshComponent|SetAnimClass _mesh "/Game/Paul/Character1/ABP_FightingAI.ABP_FightingAI_C")
      (Variables|Default|SetPlayerNumber 0)
      (Transformation|SetRelativeTransform _mesh_2 (Math|Transform|MakeTransform "0.000000,0.000000,-66.447029" "0.000000,-89.999999,0.000000" "1.000000,1.000000,1.000000") false false)
      (return))))

(fn Parameters
  (return (or (Variables|Default|GetAttacking) (Variables|Default|GetBlocking))))

(fn FMove
  (params (move :type Boolean) (Y :type Float%20%28double-precision%29))
  (bind _charactermovement (Variables|Character|GetCharacterMovement))
  (if move
    (Class|PawnMovementComponent|AddInputVector _charactermovement (* (Math|Vector|MakeVector 0.0 Y 0.0) (Variables|/Script/Engine.CharacterMovementComponent|GetMaxWalkSpeed _charactermovement)) false)))