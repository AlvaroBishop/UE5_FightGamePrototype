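; Player character for a fighting game, which picks its mesh setup, animation class and player number from whether the level is BunnyMap.
; BeginPlay adds the input mapping, fills health and registers the player with the game mode.
; Unblocked damage lowers health and sets a hurt flag, which Tick turns into a character-specific montage through a resettable DoOnce.
; HitCheck damages AI fighters overlapping a hitbox and pushes their health to the UI.
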(event EventBeginPlay
  (CallFunction|SetPlayer)
  (bind _aspc_player_controller (Utilities|Casting|CastToPC_PlayerController (Pawn|GetController)))
  (Variables|Default|SetAs%20PC%20Player%20Controller _aspc_player_controller)
  (Utilities|IsValid (PlayerController|LocalPlayerSubsystems|GetEnhancedInputLocalPlayerSubsystem _aspc_player_controller)
    (:Is%20Valid
      (Input|AddMappingContext (PlayerController|LocalPlayerSubsystems|GetEnhancedInputLocalPlayerSubsystem _aspc_player_controller) "/Game/Paul/Character1/Inputs/IMC_Player.IMC_Player" 0 "(bIgnoreAllPressedKeysUntilRelease=True,bForceImmediately=False)")
      (Variables|Default|SetCurrentHealth (Variables|Default|GetMaxHealth))
      (bind _asgm_fighting_player (Utilities|Casting|CastToGM_FightingPlayer (Game|GetGameMode)))
      (Variables|/Game/Paul/GM_FightingPlayer.GM_FightingPlayer_C|SetPlayer _asgm_fighting_player self))))

(event EventTick
  (params (DeltaSeconds :type Float%20%28single-precision%29))
  (if (Variables|Default|GetisHurt)
    (Utilities|FlowControl|DoOnce false :!label _label
      (:Completed
        (Animation|Montage|PlayMontage (Variables|Character|GetMesh) (Utilities|Select :Index (Variables|Default|GetPlayerNumber) :Option%200 "/Game/Paul/Character1/Model/Animations/Montage/TakingPunch_Montage.TakingPunch_Montage" :Option%201 "/Game/Paul/Character1/Model2/Animations/Montage/Hurt_Montage.Hurt_Montage")
          (:OnCompleted
            (Variables|Default|SetisHurt false)
            (goto _label Reset)))))))

(event Game|Damage|EventAnyDamage
  (params (Damage :type Float%20%28single-precision%29) (DamageType :type Damage%20Type%20Object%20Reference) (InstigatedBy :type Controller%20Object%20Reference) (DamageCauser :type Actor%20Object%20Reference))
  (if (not (Variables|/Game/Paul/PC_PlayerController.PC_PlayerController_C|GetBlocking (Variables|Default|GetAs%20PC%20Player%20Controller)))
    (Variables|Default|SetCurrentHealth (Math|Float|Clamp(Float) (- (Variables|Default|GetCurrentHealth) Damage) 0.0 1e+02))
    (Variables|Default|SetisHurt true)))

(fn ConstructionScript)

(fn HitCheck
  (params (InputPin :type Float%20%28single-precision%29) (HitBox :type Primitive%20Component%20Object%20Reference))
  (for _array_element (Collision|GetOverlappingActors HitBox "/Game/Paul/Character1/BP_FightingAI.BP_FightingAI_C" :!class /Script/Engine.PrimitiveComponent)
    (if (!= _array_element self)
      (Game|Damage|ApplyDamage _array_element InputPin 0 0)
      (bind _asbp_fighting_ai (Utilities|Casting|CastToBP_FightingAI _array_element))
      (Default|UpdateHealthUI (Variables|/Game/Paul/PC_PlayerController.PC_PlayerController_C|GetWB_Main (Variables|Default|GetAs%20PC%20Player%20Controller)) false (Variables|/Game/Paul/Character1/BP_FightingAI.BP_FightingAI_C|GetCurrentHealth _asbp_fighting_ai)))))

(fn CheckLevel
  (bind _returnvalue (Game|GetCurrentLevelName true))
  (return (Utilities|Enum|Equal(Enum) _returnvalue "BunnyMap")))

(fn SetPlayer
  (bind _mesh (Variables|Character|GetMesh))
  (bind _mesh_2 (Variables|Character|GetMesh))
  (if (CallFunction|CheckLevel)
    ;[1 1 1] BUNNY
    (Variables|/Script/Engine.SkeletalMeshComponent|SetSkeletalMeshAsset _mesh "/Game/Paul/Character1/Model/T-Pose.T-Pose")
    (Class|SkeletalMeshComponent|SetAnimClass _mesh "/Game/Paul/Character1/ABP_FightingPlayer.ABP_FightingPlayer_C")
    (Variables|Default|SetPlayerNumber 0)
    (Transformation|SetRelativeTransform _mesh_2 (Math|Transform|MakeTransform "0.000000,0.000000,-66.447029" "0.000000,-89.999999,0.000000" "1.000000,1.000000,1.000000") false false)
    (return)
    (else
      ;[1 1 1] BOMB
      (Variables|/Script/Engine.SkeletalMeshComponent|SetSkeletalMeshAsset _mesh "/Game/Paul/Character1/Model2/T-Pose.T-Pose")
      (Class|SkeletalMeshComponent|SetAnimClass _mesh "/Game/Paul/Character1/ABP_FightingPlayer2.ABP_FightingPlayer2_C")
      (Variables|Default|SetPlayerNumber 1)
      (Transformation|SetRelativeTransform _mesh_2 (Math|Transform|MakeTransform "0.000000,0.000000,-66.447029" "0.000000,-89.999999,0.000000" "0.500000,0.500000,0.500000") false false)
      (return))))