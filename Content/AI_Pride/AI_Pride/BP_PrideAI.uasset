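; BP_PrideAI is a sword-wielding enemy that takes damage and damages the third-person player character.
; Incoming damage lowers Health, and at zero the actor is destroyed unless it is flagged as a boss.
; TriggerSword starts a fast looping timer that line-traces between two mesh sockets, with persistent debug drawing.
; A DoOnce limits player damage to one hit per swing, and StopTriggerSword clears the timer and resets it.
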(event Custom|TriggerSword
  ;[1 1 1] Damage Player
  (bind _returnvalue (Utilities|Time|SetTimerbyEvent (delegate Custom|SwordLineTrace) 0.01 true))
  (Variables|Default|Settrigger%20sword%20event _returnvalue))

(event Custom|SwordLineTrace
  (bind _mesh (Variables|Character|GetMesh))
  ;[1 1 1] Damage Player
  (bind _outhit (Collision|LineTraceByChannel (Transformation|GetSocketLocation _mesh "start") (Transformation|GetSocketLocation _mesh "end") "TraceTypeQuery2" false 0 "Persistent"))
  (bind _asbp_third_person_character (Utilities|Casting|CastToBP_ThirdPersonCharacter (.HitActor (Collision|BreakHitResult _outhit))))
  (Utilities|FlowControl|DoOnce false
    (:Completed
      (Game|Damage|ApplyDamage _asbp_third_person_character 2.5 0 0))))

(event Custom|StopTriggerSword
  ;[1 1 1] Damage Player
  (Utilities|Time|ClearandInvalidateTimerbyHandle (Variables|Default|Gettrigger%20sword%20event))
  (Utilities|FlowControl|DoOnce false) ; enters at Reset
)

(event Game|Damage|EventAnyDamage
  (params (Damage :type Float%20%28single-precision%29) (DamageType :type Damage%20Type%20Object%20Reference) (InstigatedBy :type Controller%20Object%20Reference) (DamageCauser :type Actor%20Object%20Reference))
  ;[1 1 1] Damage
  (bind _output_get (Variables|Default|SetHealth (- (Variables|Default|GetHealth) Damage)))
  (if (<= _output_get 0.0)
    (if (not (Variables|Default|GetisBoss))
      (Actor|DestroyActor))))

(fn ConstructionScript)